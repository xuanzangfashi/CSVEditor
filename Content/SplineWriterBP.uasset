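; Spline path authoring actor that rebuilds a spline from the Cone1_tra1j data table and moves a Cube along it.
; SplineWriter adds one point per row, with XY scaled by IntervalSpace, raw z_axis as Z, and zeroed tangents.
; Tick advances the Cube by Speed over elapsed time, reusing the spline's Z, converted from radians to degrees, as yaw.
; Separate events clear the spline or export it to a fixed CSV path.
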(event Custom|SplineWriter
  (bind _returnvalue (Math|Vector|MakeVector 0.0 0.0 0.0))
  (bind _spline (Variables|Default|GetSpline))
  (Spline|ClearSplinePoints (Variables|Default|GetSpline) false)
  ;[1 0 0] INSERT SHAPE DATA TABLE HERE
  (bind _outrownames (DataTable|GetDataTableRowNames "/Game/cone1_tra1j.cone1_tra1j"))
  (for _index (range 0 (Utilities|Array|LastIndex _outrownames))
    (Spline|AddSplinePoint (Variables|Default|GetSpline) (Math|Vector|MakeVector 0.0 0.0 0.0) "World" false))
  (for _index_2 (range 0 (Utilities|Array|LastIndex _outrownames))
    ;[1 0 0] INSERT SHAPE DATA TABLE HERE
    (bind _returnvalue_2 (Utilities|GetDataTableRow "/Game/cone1_tra1j.cone1_tra1j" (Utilities|Array|Get(acopy) _outrownames _index_2))
      (:then
        (Spline|SetLocationatSplinePoint _spline _index_2 (Math|Vector|MakeVector (.X (Math|Vector|BreakVector (* (Math|Vector|MakeVector (.x _returnvalue_2) (.y _returnvalue_2) 0.0) (Variables|Default|Getinterval_space)))) (.Y (Math|Vector|BreakVector (* (Math|Vector|MakeVector (.x _returnvalue_2) (.y _returnvalue_2) 0.0) (Variables|Default|Getinterval_space)))) (.z_axis _returnvalue_2)) "World" false)
        (Spline|SetTangentsatSplinePoint _spline _index_2 _returnvalue _returnvalue "Local" true)))))

(event Custom|CustomEvent_0
  (while true
    (Spline|RemoveSplinePoint (Variables|Default|GetSpline) (Variables|Default|GetNewVar_1) true)))

(event Custom|Export_CSV
  (Class|CSVSave|SaveCurrentCsvFile "D:/1.csv" (Variables|Default|GetSpline) (Variables|Default|Getinterval_space)))

(event Custom|Clear
  (bind _spline (Variables|Default|GetSpline))
  (Spline|ClearSplinePoints _spline false)
  (Spline|AddSplinePoint _spline (Math|Vector|MakeVector 0.0 0.0 0.0) "World" false))

(event EventBeginPlay)

(event Collision|EventActorBeginOverlap
  (params (OtherActor :type Actor%20Object%20Reference)))

(event EventTick
  (params (DeltaSeconds :type Float%20%28single-precision%29))
  (Variables|Default|Settime_past (+ (Variables|Default|Gettime_past) DeltaSeconds))
  (Transformation|SetWorldLocation (Variables|Default|GetCube) (Spline|GetLocationatDistanceAlongSpline (Variables|Default|GetSpline) (* (Variables|Default|Getspeed) (Variables|Default|Gettime_past)) "World") false false)
  (Transformation|SetWorldRotation (Variables|Default|GetCube) (Math|Rotator|MakeRotator 0.0 0.0 (Math|Trig|RadiansToDegrees (.Z (Math|Vector|BreakVector (Spline|GetLocationatDistanceAlongSpline (Variables|Default|GetSpline) (* (Variables|Default|Getspeed) (Variables|Default|Gettime_past)) "World"))))) false false))

(fn ConstructionScript)